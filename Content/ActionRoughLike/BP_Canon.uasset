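; BP_Canon is a turret actor that continuously fires magic projectiles at the player.
; On BeginPlay a short looping timer spawns BP_MagicProjectile at the actor's location, using the rotation of its Arrow component.
; Each Tick rotates the Arrow toward player pawn 0 with FindLookAtRotation, so shots track the player with no range or line-of-sight check.
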(event Custom|SpawnProjectile
  (Game|SpawnActorfromClass "/Game/ActionRoughLike/Projectiles/BP_MagicProjectile.BP_MagicProjectile_C" (Math|Transform|MakeTransform (Transformation|GetActorLocation) (Transformation|GetWorldRotation (Variables|Default|GetArrow))) "Undefined" "MultiplyWithRoot" 0 0))

(event EventBeginPlay
  (Utilities|Time|SetTimerbyEvent (delegate Custom|SpawnProjectile) 0.4 true))

(event EventTick
  (params (DeltaSeconds :type Float%20%28single-precision%29))
  (Transformation|SetWorldRotation (Variables|Default|GetArrow) (Math|Rotator|FindLookatRotation (Transformation|GetActorLocation) (Transformation|GetActorLocation (Game|Player|GetPlayerPawn 0))) false false))

(fn ConstructionScript)